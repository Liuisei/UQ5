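; Enemy character Blueprint for UnrealQuest5 with HP, a widget health bar, a montage attack, and a parry reaction.
; Attack montage notifies spawn a short-lived BP_DamageP hitbox on "ATK" and set the IsATK parry window on "EATKStart".
; Damage of the matching target type lowers HP and updates the bar, interrupting the attack with a parried montage if IsATK is set.
; At zero HP, it spawns a UQ5_EnemyLagDoll in its place and destroys itself.
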(event `Attack`
  ;[1 0 0 0.5] 攻撃
  (bind _notifyname (`|PlayMontage` (`self.Mesh`) "/Game/UnrealQuest5/Characters/Mannequins/Animations/UQ5/AM_Enemy_Attack01.AM_Enemy_Attack01")
    (:`OnInterrupted`
      (set `self.IsATK` false))
    (:`OnNotifyBegin`
      (if (== _notifyname "ATK")
        (`self.SpawnATK`)
        (else
          (set `self.IsATK` (== _notifyname "EATKStart")))))))

(event `self.ReceiveBeginPlay`
  ;[1 1 1] Start
  (bind _aswbp_hpbar (cast `/Game/My/UI/WBP_HPBar` (`WidgetComponent.GetWidget` (`self.Widget`))))
  (`/Game/My/UI/WBP_HPBar.UpDateHP` _aswbp_hpbar (`self.HP`) (`self.MaxHP`)))

(event `ChangeSpeed`
  (params (`Max Walk Speed` :type "Float (single-precision)"))
  (set `CharacterMovementComponent.MaxWalkSpeed` `Max Walk Speed` (`self.CharacterMovement`)))

(event `SpawnATK`
  ;[1 1 1] Comment
  (bind _returnvalue (`|SpawnActorFromClass` "/Game/My/Bp/BP_DamageP.BP_DamageP_C" (`SceneComponent.K2_GetComponentToWorld` (`self.Scene`)) "Undefined" "MultiplyWithRoot" null 10 "NewEnumerator1" null))
  (`/Game/My/Bp/BP_DamageP.LifeTime` _returnvalue 0.2))

(event `/Game/My/Interface/BPI_Damage.Damage`
  (params (DamageValue :type Integer) (TergetType :type "/Game/My/Enum/EChalacterType Enum" :default "NewEnumerator0"))
  (bind _isatk (`self.IsATK`))
  ;[1 0.4896 0.4896] 攻撃された
  (if (`|EnumEquality` TergetType "NewEnumerator0")
    (if (not (`self.IsDie`))
      (`self.GetDamage` DamageValue)
      (bind _aswbp_hpbar (cast `/Game/My/UI/WBP_HPBar` (`WidgetComponent.GetWidget` (`self.Widget`))))
      (`/Game/My/UI/WBP_HPBar.UpDateHP` _aswbp_hpbar (`self.HP`) (`self.MaxHP`))
      (`self.Die`)
      (`KismetSystemLibrary.PrintString` (`KismetStringLibrary.Conv_BoolToString` _isatk))
      (if _isatk
        (`self.StopAnimMontage` "/Game/UnrealQuest5/Characters/Mannequins/Animations/UQ5/AM_Enemy_Attack01.AM_Enemy_Attack01")
        (`|PlayMontage` (`self.Mesh`) "/Game/UnrealQuest5/Characters/Mannequins/Animations/UQ5/AM_GotParried.AM_GotParried")))))

(event `Die`
  ;[1 1 1] Die
  (bind _output_get (set `self.IsDie` (<= (`self.HP`) 0)))
  (if _output_get
    (`/Engine/EditorBlueprintResources/StandardMacros.DoOnce` false
      (:`Completed`
        (`|SpawnActorFromClass` "/Game/UnrealQuest5/Blueprints/UQ5_EnemyLagDoll.UQ5_EnemyLagDoll_C" (`self.GetTransform` self) "Undefined" "MultiplyWithRoot" null null)
        (`self.K2_DestroyActor`)))))

(fn `GetDamage`
  (params (DamageValue :type Integer))
  (set `self.HP` (- (`self.HP`) DamageValue)))

(fn `UserConstructionScript`)