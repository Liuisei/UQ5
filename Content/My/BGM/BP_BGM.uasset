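; BP_BGM is a background music manager that plays one 2D track at a time.
; On BeginPlay it creates and plays the Xmas_Tonight sound, keeping the audio component in NowBGM.
; UpdateSound stops the current component, looks up the requested item in the Sound array, then creates and plays a new 2D component that replaces NowBGM.
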(event `self.ReceiveBeginPlay`
  (bind _returnvalue (`GameplayStatics.CreateSound2D` "/Game/My/BGM/Xmas_Tonight.Xmas_Tonight" 1.0 1.0 0.0 null))
  (bind _output_get (set `self.NowBGM` _returnvalue))
  (`AudioComponent.Play` _output_get 0.0))

(event `UpdateSound`
  (params (ItemToFind :type "SoundBase Object Reference (by ref)"))
  (bind _sound (`self.Sound`))
  (`AudioComponent.Stop` (`self.NowBGM`))
  (bind _returnvalue (`GameplayStatics.CreateSound2D` (`|GetArrayItem` _sound (`KismetArrayLibrary.Array_Find` _sound ItemToFind)) 1.0 1.0 0.0 null))
  (bind _output_get (set `self.NowBGM` _returnvalue))
  (`AudioComponent.Play` _output_get 0.0))

(fn `UserConstructionScript`)