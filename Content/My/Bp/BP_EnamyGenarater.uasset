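; Enemy generator actor that spawns random enemy classes at its donut mesh and prints a win message once all of them are gone.
; HP acts as the spawn budget: each spawn spends one point, refreshes the WBP_HPBar widget and gives the enemy its default controller.
; Spawn re-calls itself on a delay, then alternates with Spawned to prune invalid enemy references until the list is empty.
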(event `self.ReceiveBeginPlay`
  ;[1 1 1] コメント
  (`self.UpdateHP`)
  (`self.Spawn`))

(event `UpdateHP`
  ;[1 1 1] コメント
  (bind _aswbp_hpbar (cast `/Game/My/UI/WBP_HPBar` (`WidgetComponent.GetWidget` (`self.Widget`))))
  (`/Game/My/UI/WBP_HPBar.UpDateHP` _aswbp_hpbar (`self.HP`) (`self.MaxHP`)))

(event `Spawn`
  ;[1 1 1] コメント
  (if (> (`self.HP`) 0)
    (set `self.HP` (- (`self.HP`) 1))
    (bind _returnvalue (`|SpawnActorFromClass` (`KismetArrayLibrary.Array_Random` (`self.SpawnEnemys`)) (`KismetMathLibrary.MakeTransform` (`SceneComponent.K2_GetComponentLocation` (`self.SM_Donut`))) "Undefined" "MultiplyWithRoot" null null))
    (`KismetArrayLibrary.Array_Add` (`self.EnemyS`) _returnvalue)
    (`Pawn.SpawnDefaultController` _returnvalue)
    (`self.UpdateHP`)
    (`KismetSystemLibrary.Delay` 3.0)
    (`self.Spawn`)
    (else
      (`self.Spawned`))))

(event `Spawned`
  ;[1 1 1] コメント
  (for _array_element (`self.EnemyS`)
    (if (not (`KismetSystemLibrary.IsValid` _array_element))
      (`KismetArrayLibrary.Array_RemoveItem` (`self.EnemyS`) _array_element)))
  (if (== (`KismetArrayLibrary.Array_Length` (`self.EnemyS`)) 0)
    (`KismetSystemLibrary.PrintString` "YouWin")
    (else
      (`KismetSystemLibrary.Delay` 1.0)
      (`self.Spawn`))))

(fn `UserConstructionScript`)